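; Base Blueprint for player projectiles, which move through a ProjectileMovement component and react to overlaps on ProjectileMesh.
; The construction script sets initial and maximum speed from Speed and scales the actor by ProjectileScale.
; Overlaps with other player projectiles are ignored; any other actor destroys the projectile.
; ApplyDamage targets the failed cast's empty result rather than the overlapped actor, and a TODO marks the cast for replacement with an enemy class.
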(event OnComponentBeginOverlap(ProjectileMesh)
  (params (OverlappedComponent :type Primitive%20Component%20Object%20Reference) (OtherActor :type Actor%20Object%20Reference) (OtherComp :type Primitive%20Component%20Object%20Reference) (OtherBodyIndex :type Integer) (bFromSweep :type Boolean) (SweepResult :type Hit%20Result%20Structure%20%28by%20ref%29))
  ;[1 1 1] Collision Event
  ;;[1 0 0.2362] TODO Replace with ENEMY
  (bind _asbp_projectile_player_base (Utilities|Casting|CastTobpProjectilePlayerBase OtherActor)
    (:CastFailed
      (Game|Damage|ApplyDamage _asbp_projectile_player_base (Variables|Default|GetDamage) 0 0)
      (Actor|DestroyActor))))

(fn ConstructionScript
  (bind _projectilemovement (Variables|Default|GetProjectileMovement))
  (bind _output_get (Variables|/Script/Engine.ProjectileMovementComponent|SetInitialSpeed _projectilemovement (Variables|Default|GetSpeed)))
  (Variables|/Script/Engine.ProjectileMovementComponent|SetMaxSpeed _projectilemovement _output_get)
  (Transformation|SetActorScale3D (Variables|Default|GetProjectileScale)))